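; Projectile actor that resolves hits between the player and AI characters, using a FiredByAI flag to tell sides apart.
; On overlap, player shots spawn an explosion, destroy the AI character and increment the player's kill count.
; AI shots slightly reduce player health and spawn an explosion.
; The projectile destroys itself after a fixed delay; the Weapon destroy on AI kills relies on a cast that never executes.
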(event EventBeginPlay
  (Utilities|FlowControl|Delay 4.0)
  (Actor|DestroyActor))

(event Collision|EventActorBeginOverlap
  (params (OtherActor :type Actor%20Object%20Reference))
  (bind _asai_character (Utilities|Casting|CastToAI_Character OtherActor)
    (:then
      (if (not (Variables|Default|GetFiredByAI))
        (Game|SpawnActorfromClass "/Game/StarterContent/Blueprints/Blueprint_Effect_Explosion.Blueprint_Effect_Explosion_C" (Math|Conversions|ToTransform(Vector) (Transformation|GetActorLocation _asai_character)) "AlwaysSpawn" 0 0)
        (Actor|DestroyActor (stale _asweapon))
        (Actor|DestroyActor _asai_character)
        (bind _asue_4asp_character (Utilities|Casting|CastToUe4ASP_Character (Game|GetPlayerCharacter 0)))
        (bind _result (Math|Integer|IncrementInt (Variables|/Game/PlayerCharacter/Ue4ASP_Character.Ue4ASP_Character_C|GetAiKilled _asue_4asp_character))
          (:%20%20
            (Variables|/Game/PlayerCharacter/Ue4ASP_Character.Ue4ASP_Character_C|SetAiKilled _asue_4asp_character _result)))))
    (:CastFailed
      (bind _asue_4asp_character_2 (Utilities|Casting|CastToUe4ASP_Character OtherActor))
      (if (Variables|Default|GetFiredByAI)
        (Variables|/Game/PlayerCharacter/Ue4ASP_Character.Ue4ASP_Character_C|SetHealth _asue_4asp_character_2 (- (Variables|/Game/PlayerCharacter/Ue4ASP_Character.Ue4ASP_Character_C|GetHealth _asue_4asp_character_2) 0.01))
        (Game|SpawnActorfromClass "/Game/StarterContent/Blueprints/Blueprint_Effect_Explosion.Blueprint_Effect_Explosion_C" (Math|Conversions|ToTransform(Vector) (Transformation|GetActorLocation _asue_4asp_character_2)) "AlwaysSpawn" 0 0)))))

(fn ConstructionScript)